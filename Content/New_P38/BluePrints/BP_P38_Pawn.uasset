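; Player-controlled P-38 aircraft pawn with flight controls, boost, braking and rocket fire.
; Roll, pitch and yaw axes apply local rotation per frame without delta-time scaling, while Tick spins both propellers and feeds forward movement input scaled by the Acceleration axis.
; Boost and Deceleration actions adjust FloatingPawnMovement limits while held, with Boost also scaling acceleration input.
; Fire spawns BP_Rocket at the Arrow component's transform.
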(event `InputAxis|Roll`
  (params (AxisValue :type "Float (single-precision)"))
  (`self.K2_AddActorLocalRotation` (`KismetMathLibrary.MakeRotator` (* AxisValue 0.5))))

(event `InputAxis|Pitch`
  (params (AxisValue :type "Float (single-precision)"))
  (`self.K2_AddActorLocalRotation` (`KismetMathLibrary.MakeRotator` 0.0 (* AxisValue 0.5))))

(event `InputAxis|Yaw`
  (params (AxisValue :type "Float (single-precision)"))
  (`self.K2_AddActorLocalRotation` (`KismetMathLibrary.MakeRotator` 0.0 0.0 (* AxisValue 0.5))))

(event `self.ReceiveTick`
  (params (DeltaSeconds :type "Float (single-precision)"))
  (`SceneComponent.K2_AddLocalRotation` (`self.PropellerRight`) (`KismetMathLibrary.MakeRotator` (* (`GameplayStatics.GetWorldDeltaSeconds`) (`self.PropellerRotationSpeed`))) false false)
  (`SceneComponent.K2_AddLocalRotation` (`self.PropellerLeft`) (`KismetMathLibrary.MakeRotator` (* (`GameplayStatics.GetWorldDeltaSeconds`) (`self.PropellerRotationSpeed`))) false false)
  (`self.AddMovementInput` (`self.GetActorForwardVector`) (`self.MoveSpeed`)))

(event `InputAxis|Acceleration`
  (params (AxisValue :type "Float (single-precision)"))
  (set `self.MoveSpeed` (* AxisValue (`self.BoostAccel`))))

(event `InputAction|Deceleration`
  (params (Key :type "Key Structure"))
  (bind _floatingpawnmovement (`self.FloatingPawnMovement`))
  (:`Pressed`
    (set `FloatingPawnMovement.Deceleration` 300.0 _floatingpawnmovement))
  (:`Released`
    (set `FloatingPawnMovement.Deceleration` 150.0 _floatingpawnmovement)))

(event `InputAction|Fire`
  (params (Key :type "Key Structure"))
  (:`Pressed`
    (`|SpawnActorFromClass` "/Game/New_P38/BluePrints/BP_Rocket.BP_Rocket_C" (`SceneComponent.K2_GetComponentToWorld` (`self.Arrow`)) "Undefined" "OverrideRootScale" null null)))

(event `InputAction|Boost`
  (params (Key :type "Key Structure"))
  (bind _floatingpawnmovement (`self.FloatingPawnMovement`))
  (:`Pressed`
    (set `self.BoostAccel` 1.5)
    (set `FloatingPawnMovement.MaxSpeed` 1800.0 _floatingpawnmovement))
  (:`Released`
    (set `self.BoostAccel` 1.0)
    (set `FloatingPawnMovement.MaxSpeed` 1200.0 _floatingpawnmovement)))

(fn `UserConstructionScript`)